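; Swinging door prop that opens while an actor overlaps it and closes when overlap ends, with optional key locking.
; A locked door checks the overlapping actor's Inventory component for KeyIndex, unlocks permanently if found, and prints key-used, key-needed or locked messages.
; Tick calls Open or Close based on IsOpen, stepping the door's relative yaw by Speed and delta time, clamped between Angle and zero.
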(event Collision|EventActorBeginOverlap
  (params (OtherActor :type Actor%20Object%20Reference))
  (bind _returnvalue (Actor|GetComponentbyClass OtherActor "/Game/FPS/Inventory/Inventory.Inventory_C"))
  (bind _key_needed (Variables|Default|GetKey%20Needed))
  (bind _key_needed_2 (Variables|Default|GetKey%20Needed))
  (if (Variables|Default|GetIsLocked)
    (Utilities|IsValid _returnvalue
      (:Is%20Valid
        (bind _has_item (Default|HasItem _returnvalue (Variables|Default|GetKeyIndex)))
        (if _has_item
          (Variables|Default|SetIsOpen true)
          (Variables|Default|SetIsLocked false)
          (if (Utilities|Enum|NotEqual(Enum) _key_needed "")
            (Development|PrintString (Utilities|String|Append _key_needed " used.") true true "(R=1.000000,G=0.000000,B=0.000000,A=1.000000)" 5.0)
            (else
              (Development|PrintString "Door is Locked!" true true "(R=1.000000,G=0.000000,B=0.000000,A=1.000000)" 5.0)))
          (elif (Utilities|Enum|NotEqual(Enum) _key_needed_2 "")
            (Development|PrintString (Utilities|String|Append _key_needed_2 " Needed!") true true "(R=1.000000,G=0.000000,B=0.000000,A=1.000000)" 5.0)
            (else
              (Development|PrintString "Door is Locked!" true true "(R=1.000000,G=0.000000,B=0.000000,A=1.000000)" 5.0))))))
    (else
      (Variables|Default|SetIsOpen true))))

(event EventTick
  (params (DeltaSeconds :type Float%20%28single-precision%29))
  (if (Variables|Default|GetIsOpen)
    (CallFunction|Open DeltaSeconds)
    (else
      (CallFunction|Close DeltaSeconds))))

(event Collision|EventActorEndOverlap
  (params (OtherActor :type Actor%20Object%20Reference))
  (Variables|Default|SetIsOpen false))

(fn ConstructionScript)

(fn Open
  (params (Delta%20Seconds :type Float%20%28single-precision%29))
  (bind _door (Variables|Default|GetDoor))
  (Transformation|SetRelativeRotation _door (Math|Rotator|MakeRotator 0.0 0.0 (Math|Float|Clamp(Float) (+ (.yaw (Variables|/Script/Engine.SceneComponent|GetRelativeRotation _door)) (* (Variables|Default|GetSpeed) Delta%20Seconds)) (Variables|Default|GetAngle) 0.0)) false false))

(fn Close
  (params (Delta%20Seconds :type Float%20%28single-precision%29))
  (bind _door (Variables|Default|GetDoor))
  (Transformation|SetRelativeRotation _door (Math|Rotator|MakeRotator 0.0 0.0 (Math|Float|Clamp(Float) (- (.yaw (Variables|/Script/Engine.SceneComponent|GetRelativeRotation _door)) (* (Variables|Default|GetSpeed) Delta%20Seconds)) (Variables|Default|GetAngle) 0.0)) false false))