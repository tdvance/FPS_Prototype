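; FPS_PlayerController is the player controller for an FPS game that toggles a Settings menu with the O or Escape key.
; Both keys share one FlipFlop that alternates between opening and closing the menu.
; Opening creates a new Settings widget, shows the cursor and sets Game and UI input.
; Closing restores game-only input, hides the cursor and removes all widgets, not just the menu.
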(event Input|KeyboardEvents|O
  (params (Key :type Key%20Structure :default "AnyKey"))
  (bind _returnvalue (Game|GetPlayerController 0))
  (:Pressed
    (Utilities|FlowControl|FlipFlop
      (:A
        (Input|SetInputModeGameandUI self 0 "LockOnCapture" true)
        (Variables|Default|SetbShowMouseCursor true)
        (bind _returnvalue_2 (UserInterface|CreateWidget "/Game/FPS/Game/UI/Settings.Settings_C"))
        (UserInterface|Viewport|AddtoViewport _returnvalue_2 0))
      (:B
        (Input|SetInputModeGameOnly _returnvalue)
        (Viewport|RemoveAllWidgets)
        (Variables|/Script/Engine.PlayerController|SetbShowMouseCursor _returnvalue false)))))

(event Input|KeyboardEvents|Escape
  (params (Key :type Key%20Structure :default "AnyKey"))
  (bind _returnvalue (Game|GetPlayerController 0))
  (:Pressed
    (Utilities|FlowControl|FlipFlop
      (:A
        (Input|SetInputModeGameandUI self 0 "LockOnCapture" true)
        (Variables|Default|SetbShowMouseCursor true)
        (bind _returnvalue_2 (UserInterface|CreateWidget "/Game/FPS/Game/UI/Settings.Settings_C"))
        (UserInterface|Viewport|AddtoViewport _returnvalue_2 0))
      (:B
        (Input|SetInputModeGameOnly _returnvalue)
        (Viewport|RemoveAllWidgets)
        (Variables|/Script/Engine.PlayerController|SetbShowMouseCursor _returnvalue false)))))

(fn ConstructionScript)