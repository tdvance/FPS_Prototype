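; FPS HUD Blueprint that draws a bottom status bar showing the player's health, armor and current ammo.
; Each DrawHUD event draws a background texture strip across the bottom of the screen, then casts the owning controller's pawn to Player.
; Health and armor come from the player's Stats, and ammo from its Inventory for the current gun, each drawn as colored, rounded text placed by screen-size fractions.
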(event EventDrawHUD
  (params (SizeX :type Integer) (SizeY :type Integer))
  (CallFunction|DrawHudTexture SizeX SizeY)
  (bind _asplayer (CallFunction|GetPlayer))
  (CallFunction|DrawCurrentAmmo SizeX SizeY _asplayer)
  (CallFunction|DrawHealth SizeX SizeY _asplayer)
  (CallFunction|DrawArmor SizeX SizeY _asplayer))

(fn ConstructionScript)

(fn DrawHudTexture
  (params (X :type Integer) (Y :type Integer))
  (Canvas|DrawTexture (Variables|Default|GetHudTexture) (* X 0.0) (* Y 0.9) (* X 1.0) (* Y 0.1) 0.0 0.0 1.0 1.0 "(R=1.000000,G=1.000000,B=1.000000,A=1.000000)"))

(fn GetPlayer
  (bind _asplayer (Utilities|Casting|CastToPlayer (Pawn|GetControlledPawn (Game|Player|GetOwningPlayerController))))
  (return _asplayer))

(fn DrawCurrentAmmo
  (params (X :type Integer) (Y :type Integer) (Player :type Player%20Object%20Reference))
  (bind _amount (Default|GetAmount (Variables|/Game/FPS/Player/Player.Player_C|GetInventory Player) (Variables|/Game/FPS/Player/Player.Player_C|GetCurrentGun Player)))
  (HUD|DrawText (Utilities|String|ToString(Integer) (Math|Float|Round _amount)) "(R=1.000000,G=0.000000,B=0.000000,A=1.000000)" (* X 0.68) (* Y 0.935) 0 3.0 false))

(fn DrawHealth
  (params (X :type Integer) (Y :type Integer) (Player :type Player%20Object%20Reference))
  (HUD|DrawText (Utilities|String|ToString(Integer) (Math|Float|Round (Default|GetHealth (Variables|/Game/FPS/Player/Player.Player_C|GetStats Player)))) "(R=0.000000,G=0.629000,B=1.000000,A=1.000000)" (* X 0.08) (* Y 0.935) 0 3.0 false))

(fn DrawArmor
  (params (X :type Integer) (Y :type Integer) (Player :type Player%20Object%20Reference))
  (HUD|DrawText (Utilities|String|ToString(Integer) (Math|Float|Round (Default|GetShielding (Variables|/Game/FPS/Player/Player.Player_C|GetStats Player)))) "(R=1.000000,G=0.767290,B=0.012887,A=1.000000)" (* X 0.25) (* Y 0.935) 0 3.0 false))