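; Utility function library for the FPS game, giving shared helpers for on-screen messages, actor counts and game mode data.
; DisplayMessage passes text and color to the first top-level Messages widget it finds, without checking that one exists.
; CountActors returns how many actors of a class are in the world.
; GetLevelStats and GetEndCamera forward to FPS_Gamemode through a cast of the current game mode.
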(fn DisplayMessage
  (params (Message :type String) (Text%20Color%20 :type Linear%20Color%20Structure :default "(SpecifiedColor=(R=0.000000,G=0.191309,B=1.000000,A=1.000000),ColorUseRule=UseColor_Specified)"))
  (bind _foundwidgets (Widget|GetAllWidgetsOfClass (LocalVariables|Get__WorldContext) "/Game/FPS/Game/UI/Messages.Messages_C"))
  (Default|SetMessage (Utilities|Array|Get(acopy) _foundwidgets) (Utilities|Text|ToText(String) Message) Text%20Color%20))

(fn CountActors
  (params (ActorClass :type Actor%20Class%20Reference))
  (bind _outactors (Actor|GetAllActorsOfClass (LocalVariables|Get__WorldContext) ActorClass))
  (return (Utilities|Array|Length _outactors)))

(fn GetLevelStats
  (bind _asfps_gamemode (Utilities|Casting|CastToFPS_Gamemode (Game|GetGameMode (LocalVariables|Get__WorldContext))))
  (return (Default|GetLevelStats _asfps_gamemode)))

(fn GetEndCamera
  (bind _asfps_gamemode (Utilities|Casting|CastToFPS_Gamemode (Game|GetGameMode (LocalVariables|Get__WorldContext))))
  (return (Default|GetEndCamera _asfps_gamemode)))