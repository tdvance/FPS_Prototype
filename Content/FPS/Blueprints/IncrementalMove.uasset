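; IncrementalMove is a component that moves itself between a list of target actors, stepping forward or back with wraparound through NextTarget and PreviousTarget.
; On BeginPlay it falls back to its owner if no targets are set, clamps the start index and snaps to that target.
; Each tick it eases its world transform toward the current target's transform with TInterpTo at a scaled Speed, following targets that move.
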(event Custom|PreviousTarget
  (bind _targets (Variables|Default|GetTargets))
  (bind _returnvalue (Utilities|Array|Length _targets))
  (Variables|Default|SetIndex (Math|Integer|%(Integer) (+ (Variables|Default|GetIndex) (- _returnvalue 1)) _returnvalue)))

(event Custom|NextTarget
  (Variables|Default|SetIndex (Math|Integer|%(Integer) (+ (Variables|Default|GetIndex) 1) (Utilities|Array|Length (Variables|Default|GetTargets)))))

(event EventBeginPlay
  (if (<= (Utilities|Array|Length (Variables|Default|GetTargets)) 0)
    (CallFunction|SetDefaultTarget))
  (CallFunction|ClampStartIndex)
  (Variables|Default|SetIndex (Variables|Default|GetStart%20Index))
  (CallFunction|ImmediatelyMovetoIndex))

(event EventTick
  (params (DeltaSeconds :type Float%20%28single-precision%29))
  (CallFunction|MovetoIndexatSpeed DeltaSeconds))

(fn SetDefaultTarget
  (Utilities|Array|SetArrayElem (Variables|Default|GetTargets) 0 (Components|GetOwner) true)
  (Variables|Default|SetStart%20Index 0))

(fn ClampStartIndex
  (Variables|Default|SetStart%20Index (Math|Integer|Clamp(Integer) (Variables|Default|GetStart%20Index) 0 (- (Utilities|Array|Length (Variables|Default|GetTargets)) 1))))

(fn ImmediatelyMovetoIndex
  (Transformation|SetWorldTransform (Transformation|GetActorTransform (Utilities|Array|Get(acopy) (Variables|Default|GetTargets) (Variables|Default|GetIndex))) false false))

(fn MovetoIndexatSpeed
  (params (DeltaTime :type Float%20%28single-precision%29))
  (Transformation|SetWorldTransform (Class|KismetMathLibrary|TInterpto (Transformation|GetWorldTransform) (Transformation|GetActorTransform (Utilities|Array|Get(acopy) (Variables|Default|GetTargets) (Variables|Default|GetIndex))) DeltaTime (* (Variables|Default|GetSpeed) 0.05)) false false))