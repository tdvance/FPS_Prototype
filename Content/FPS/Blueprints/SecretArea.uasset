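; SecretArea is a trigger actor marking a hidden secret in an FPS level.
; On the first overlap by an actor with the triggering tag, it registers the secret with the level stats and displays a colored message showing found versus total secrets.
; A one-shot flag prevents repeat counting, and the construction script mirrors the message text onto a text render component.
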(event Collision|EventActorBeginOverlap
  (params (OtherActor :type Actor%20Object%20Reference))
  (bind _levelstats (CallFunction|GetLevelStats))
  (if (and (Actor|ActorHasTag OtherActor (Variables|Default|GetTriggeringActorTag)) (not (Variables|Default|GetHasBeenTriggered)))
    (Variables|Default|SetHasBeenTriggered true)
    (Default|AddSecretFound _levelstats)
    (CallFunction|DisplayMessage (Utilities|String|Append (Variables|Default|GetText) " (" (Utilities|String|ToString(Integer) (Variables|/Game/FPS/Blueprints/LevelStats.LevelStats_C|GetNumSecretsFound _levelstats)) "/" (Utilities|String|ToString(Integer) (Variables|/Game/FPS/Blueprints/LevelStats.LevelStats_C|GetNumSecrets _levelstats)) ")") "(R=0.000000,G=0.913945,B=1.000000,A=1.000000)")))

(fn ConstructionScript
  (Rendering|Components|TextRender|SetText (Variables|Default|GetTextRender) (Utilities|Text|ToText(String) (Variables|Default|GetText))))