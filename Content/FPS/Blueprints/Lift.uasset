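; Lift component that moves its owning actor between a list of target actors, serving as an elevator or moving platform.
; On begin play it snaps the owner to a clamped start index, using the owner itself as target when the list is empty.
; Up/next and down/previous events step the index with wraparound.
; Every tick interpolates the owner's full transform toward the current target at a scaled speed, easing into each stop.
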(event Custom|DownOrPrevious
  (bind _targets (Variables|Default|GetTargets))
  (bind _returnvalue (Utilities|Array|Length _targets))
  (Variables|Default|SetIndex (Math|Integer|%(Integer) (+ (Variables|Default|GetIndex) (- _returnvalue 1)) _returnvalue)))

(event Custom|UpOrNext
  (Variables|Default|SetIndex (Math|Integer|%(Integer) (+ (Variables|Default|GetIndex) 1) (Utilities|Array|Length (Variables|Default|GetTargets)))))

(event EventBeginPlay
  (bind _returnvalue (Components|GetOwner))
  (if (<= (Utilities|Array|Length (Variables|Default|GetTargets)) 0)
    (Utilities|Array|SetArrayElem (Variables|Default|GetTargets) 0 _returnvalue true)
    (Variables|Default|SetStart%20Index 0)
    (else
      (Variables|Default|SetStart%20Index (Math|Integer|Clamp(Integer) (Variables|Default|GetStart%20Index) 0 (- (Utilities|Array|Length (Variables|Default|GetTargets)) 1)))))
  (Variables|Default|SetIndex (Variables|Default|GetStart%20Index))
  (Transformation|SetActorTransform _returnvalue (Transformation|GetActorTransform (Utilities|Array|Get(acopy) (Variables|Default|GetTargets) (Variables|Default|GetIndex)))))

(event EventTick
  (params (DeltaSeconds :type Float%20%28single-precision%29))
  (bind _returnvalue (Components|GetOwner))
  (Transformation|SetActorTransform _returnvalue (Class|KismetMathLibrary|TInterpto (Transformation|GetActorTransform _returnvalue) (Transformation|GetActorTransform (Utilities|Array|Get(acopy) (Variables|Default|GetTargets) (Variables|Default|GetIndex))) DeltaSeconds (* (Variables|Default|GetSpeed) 0.05))))