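; FPS inventory that stores item classes in indexed slots, with a name, amount, max and super max kept in parallel arrays.
; AddNewItem defines a slot, zeroing the amount only if it was empty, and HasItem guards the getters and amount changes.
; AddToExistingItem caps at max, or super max when IgnoreMax is set, without lowering the current amount.
; UseItem deducts up to what is available and returns the amount used.
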(fn HasItem
  (params (Index :type Integer))
  (bind _items (Variables|Default|GetItems))
  (if (< Index (Utilities|Array|Length _items))
    (return (Utilities|IsValidClass (Utilities|Array|Get(acopy) _items Index)))
    (else
      (return false))))

(fn GetAmount
  (params (Index :type Integer))
  (bind _has_item (CallFunction|HasItem Index))
  (if _has_item
    (return (Utilities|Array|Get(acopy) (Variables|Default|GetAmount) Index))
    (else
      (return 0.0))))

(fn GetMaxAmount
  (params (Index :type Integer))
  (bind _has_item (CallFunction|HasItem Index))
  (return (select _has_item (Utilities|Array|Get(acopy) (Variables|Default|GetMaxAmount) Index) 0.0)))

(fn GetName
  (params (Index :type Integer))
  (bind _has_item (CallFunction|HasItem Index))
  (return (select _has_item (Utilities|Array|Get(acopy) (Variables|Default|GetNames) Index) "--")))

(fn AddtoExistingItem
  (params (Index :type Integer) (Amount :type Float%20%28single-precision%29) (IgnoreMax :type Boolean))
  (bind _output (Utilities|Array|Get(acopy) (Variables|Default|GetAmount) Index))
  (bind _has_item (CallFunction|HasItem Index))
  (if _has_item
    (LocalVariables|SetOldAmount _output)
    (Utilities|Array|SetArrayElem (Variables|Default|GetAmount) Index (CallFunction|ClamptoMax _output (+ _output Amount) (Utilities|Array|Get(acopy) (Variables|Default|GetMaxAmount) Index) (Utilities|Array|Get(acopy) (Variables|Default|GetSuperMaxAmount) Index) IgnoreMax) true)
    (return (!= (Utilities|Array|Get(acopy) (Variables|Default|GetAmount) Index) (LocalVariables|GetOldAmount)))
    (else
      (return false))))

(fn ClamptoMax
  (params (Min :type Float%20%28single-precision%29) (Amount :type Float%20%28single-precision%29) (Max :type Float%20%28single-precision%29) (SuperMax :type Float%20%28single-precision%29) (IgnoreMax :type Boolean))
  (return (Math|Float|Max(Float) (Math|Float|Clamp(Float) Amount Min (select IgnoreMax SuperMax Max)) Min)))

(fn AddNewItem
  (params (Item :type Actor%20Class%20Reference) (MaxAmount :type Float%20%28single-precision%29) (SuperMaxAmount :type Float%20%28single-precision%29) (Name :type String) (Index :type Integer))
  (bind _has_item (CallFunction|HasItem Index))
  (if _has_item
    _
    (else
      (Utilities|Array|SetArrayElem (Variables|Default|GetAmount) Index (LocalVariables|GetZero) true)))
  (Utilities|Array|SetArrayElem (Variables|Default|GetItems) Index Item true)
  (Utilities|Array|SetArrayElem (Variables|Default|GetMaxAmount) Index MaxAmount true)
  (Utilities|Array|SetArrayElem (Variables|Default|GetSuperMaxAmount) Index SuperMaxAmount true)
  (Utilities|Array|SetArrayElem (Variables|Default|GetNames) Index Name true))

(fn UseItem
  (params (Index :type Integer) (Amount :type Float%20%28single-precision%29))
  (bind _output (Utilities|Array|Get(acopy) (Variables|Default|GetAmount) Index))
  (bind _has_item (CallFunction|HasItem Index))
  (if _has_item
    (LocalVariables|SetAmountUsed (Math|Float|Clamp(Float) Amount 0.0 _output))
    (Utilities|Array|SetArrayElem (Variables|Default|GetAmount) Index (- _output (LocalVariables|GetAmountUsed)))
    (return (LocalVariables|GetAmountUsed) true)
    (else
      (return 0.0 false))))

(fn GetItem
  (params (Index :type Integer))
  (bind _has_item (CallFunction|HasItem Index))
  (if _has_item
    (return (Utilities|Array|Get(acopy) (Variables|Default|GetItems) Index))
    (else
      (return 0))))