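; Stats component for an FPS that tracks its owner's health and shielding, and sends DieMessage when health runs out.
; Damage splits by shield fill ratio, capped at full absorption, with the health share computed from the already reduced shield.
; AddHealth and AddShielding cap at a normal or super maximum via IgnoreMax, never lower an overcharged value, and report whether it changed.
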(fn ApplyDamage
  (params (Amount :type Float%20%28single-precision%29))
  (bind (_appliedtohealth _appliedtoshield) (CallFunction|ComputeShieldDamage Amount))
  (Variables|Default|SetShielding (- (Variables|Default|GetShielding) (Math|Float|Clamp(Float) _appliedtoshield 0.0 (Variables|Default|GetShielding))))
  (bind _output_get (Variables|Default|SetHealth (Math|Float|Clamp(Float) (- (Variables|Default|GetHealth) _appliedtohealth) 0.0 (Variables|Default|GetHealth))))
  (if (<= _output_get 0.0)
    (Class|GamePawn|Die(Message) (Components|GetOwner))))

(fn GetHealth
  (return (Variables|Default|GetHealth)))

(fn GetShielding
  (return (Variables|Default|GetShielding)))

(fn AddHealth
  (params (Amount :type Float%20%28single-precision%29) (IgnoreMax :type Boolean))
  (bind _health (CallFunction|GetHealth))
  (bind _maxhealth (Variables|Default|GetMaxHealth))
  (bind _supermaxhealth (Variables|Default|GetSuperMaxHealth))
  (bind _returnvalue (+ Amount _health))
  (bind _clamped (CallFunction|ClamptoMax _health _returnvalue _maxhealth _supermaxhealth IgnoreMax))
  (LocalVariables|SetOldValue _health)
  (Variables|Default|SetHealth _clamped)
  (return (!= _clamped (LocalVariables|GetOldValue))))

(fn AddShielding
  (params (Amount :type Float%20%28single-precision%29) (IgnoreMax :type Boolean))
  (bind _shielding (CallFunction|GetShielding))
  (bind _maxshielding (Variables|Default|GetMaxShielding))
  (bind _supermaxshielding (Variables|Default|GetSuperMaxShielding))
  (bind _returnvalue (+ Amount _shielding))
  (bind _clamped (CallFunction|ClamptoMax _shielding _returnvalue _maxshielding _supermaxshielding IgnoreMax))
  (LocalVariables|SetOldValue _shielding)
  (Variables|Default|SetShielding _clamped)
  (return (!= _clamped (LocalVariables|GetOldValue))))

(fn ClamptoMax
  (params (Min :type Float%20%28single-precision%29) (Amount :type Float%20%28single-precision%29) (Max :type Float%20%28single-precision%29) (SuperMax :type Float%20%28single-precision%29) (IgnoreMax :type Boolean))
  (return (Math|Float|Max(Float) (Math|Float|Clamp(Float) Amount Min (select IgnoreMax SuperMax Max)) Min)))

(fn ComputeShieldDamage
  (params (DamageAmount :type Float%20%28single-precision%29))
  (bind _shielding (Variables|Default|GetShielding))
  (bind _maxshielding (Variables|Default|GetMaxShielding))
  (bind _returnvalue (/ _shielding _maxshielding))
  (bind _returnvalue_2 (>= _returnvalue 1.0))
  (bind _returnvalue_3 (select _returnvalue_2 1.0 _returnvalue))
  (return (* DamageAmount (- 1.0 _returnvalue_3)) (* DamageAmount _returnvalue_3)))