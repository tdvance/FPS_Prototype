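; LevelStats is an actor that tracks secret and enemy totals and progress for a level in the FPS game.
; On BeginPlay it counts the SecretArea and EnemyPawnBase actors to set the secret and enemy totals.
; AddSecretFound and AddEnemyKilled each increment a running counter for secrets found and enemies killed.
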(event EventBeginPlay
  (bind _count (CallFunction|CountActors "/Game/FPS/Blueprints/SecretArea.SecretArea_C"))
  (Variables|Default|SetNumSecrets _count)
  (bind _count_2 (CallFunction|CountActors "/Game/FPS/Enemies/EnemyPawnBase.EnemyPawnBase_C"))
  (Variables|Default|SetNumEnemies _count_2))

(fn ConstructionScript)

(fn AddSecretFound
  (Variables|Default|SetNumSecretsFound (+ (Variables|Default|GetNumSecretsFound) 1)))

(fn AddEnemyKilled
  (Variables|Default|SetNumEnemiesKilled (+ (Variables|Default|GetNumEnemiesKilled) 1)))